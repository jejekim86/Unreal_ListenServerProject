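; Behavior tree service for monster AI that decides when the chase target becomes an attack target.
; Each tick it asks BP_MyEnemyCharacter whether the ChaseTarget blackboard actor is in attack range, copying it to AttackTarget if so.
; Out of range, it clears AttackTarget and resets the enemy's IsAttack flag.
; An invalid chase target clears only ChaseTarget, leaving AttackTarget untouched.
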(event `self.ReceiveTickAI`
  (params (OwnerController :type "AIController Object Reference") (ControlledPawn :type "Pawn Object Reference") (DeltaSeconds :type "Float (single-precision)"))
  (bind _returnvalue (`AIBlueprintHelperLibrary.GetBlackboard` OwnerController))
  (bind _returnvalue_2 (`KismetStringLibrary.Conv_StringToName` "AttackTarget"))
  (bind _returnvalue_3 (`KismetStringLibrary.Conv_StringToName` "ChaseTarget"))
  (bind _returnvalue_4 (`BlackboardComponent.GetValueAsObject` _returnvalue _returnvalue_3))
  (bind _asbp_my_enemy_character (cast `/Game/BP/Monster/BP_MyEnemyCharacter` ControlledPawn))
  (`/Engine/EditorBlueprintResources/StandardMacros.IsValid` _returnvalue_4
    (:`Is Valid`
      (bind _asactor (cast `Actor` _returnvalue_4))
      (bind _returnvalue_5 (`MyEnemyCharacter.IsInAttackRange` _asbp_my_enemy_character _asactor))
      (if _returnvalue_5
        (`BlackboardComponent.SetValueAsObject` _returnvalue _returnvalue_2 _returnvalue_4)
        (else
          (`BlackboardComponent.ClearValue` _returnvalue _returnvalue_2)
          (if (`MyEnemyCharacter.bIsAttack` _asbp_my_enemy_character)
            (set `MyEnemyCharacter.bIsAttack` false _asbp_my_enemy_character)))))
    (:`Is Not Valid`
      (`BlackboardComponent.ClearValue` _returnvalue _returnvalue_3))))